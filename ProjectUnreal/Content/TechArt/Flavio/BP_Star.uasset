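; BP_Star is an actor that toggles a Niagara effect based on the cabin state of a Bille object.
; The effect starts deactivated on BeginPlay.
; Each Tick polls Bille's CabaneIn flag to activate it, and deactivates it only when CabaneOut is also set while CabaneIn is true.
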(event EventBeginPlay
  (Components|Activation|Deactivate (Variables|Default|GetNiagara1)))

(event Collision|EventActorBeginOverlap
  (params (OtherActor :type Actor%20Object%20Reference)))

(event EventTick
  (params (DeltaSeconds :type Float%20%28single-precision%29))
  (bind _bille (Variables|Default|Getbille))
  (if (Variables|/Game/Blueprints/Gameplay/Pawn/BP_GAMEPLAY_Bille.BP_GAMEPLAY_Bille_C|GetCabane_in? _bille)
    (Components|Activation|Activate (Variables|Default|GetNiagara1) false)
    (if (Variables|/Game/Blueprints/Gameplay/Pawn/BP_GAMEPLAY_Bille.BP_GAMEPLAY_Bille_C|GetCabane_Out? _bille)
      (Components|Activation|Deactivate (Variables|Default|GetNiagara1)))))

(fn ConstructionScript)