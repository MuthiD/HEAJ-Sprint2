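; Cloud actor that drifts and turns its Cloud component procedurally, with a randomly picked material.
; BeginPlay rolls six random values and picks the material; RandomInteger(2) only yields 0 or 1, so CloudMat03 is never used.
; Tick feeds time-based sine waves into relative location and an X-vector-derived rotation, reusing the random values as both speed variations and offsets to vary each instance.
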(event EventBeginPlay
  (bind _cloud (Variables|Default|GetCloud))
  (Variables|Default|SetRandom (+ (* (Math|Random|RandomFloat) 1.0) 1.0))
  (Variables|Default|SetRandom_0 (+ (* (Math|Random|RandomFloat) 1.0) 1.0))
  (Variables|Default|SetRandom_2 (+ (* (Math|Random|RandomFloat) 1.0) 1.0))
  (Variables|Default|SetRandom_3 (+ (* (Math|Random|RandomFloat) 1.0) 1.0))
  (Variables|Default|SetRandom_4 (+ (* (Math|Random|RandomFloat) 1.0) 1.0))
  (Variables|Default|SetRandom_1 (+ (* (Math|Random|RandomFloat) 1.0) 1.0))
  (switch int (Math|Random|RandomInteger 2)
    (:0
      (Rendering|Material|SetMaterial _cloud 0 (Variables|Default|GetCloudMat01)))
    (:1
      (Rendering|Material|SetMaterial _cloud 0 (Variables|Default|GetCloudMat02)))
    (:2
      (Rendering|Material|SetMaterial _cloud 0 (Variables|Default|GetCloudMat03)))))

(event EventTick
  (params (DeltaSeconds :type Float%20%28single-precision%29))
  (bind _cloud (Variables|Default|GetCloud))
  (bind _rotationspeed (Variables|Default|GetRotationSpeed))
  (bind _offsetspeed (Variables|Default|GetOffsetSpeed))
  (Transformation|SetRelativeLocation _cloud (* (+ (Math|Vector|MakeVector (Math|Trig|Sin(Degrees) (* (Actor|GetGameTimeSinceCreation) (+ _offsetspeed (Variables|Default|GetRandom)))) (Math|Trig|Sin(Degrees) (* (Actor|GetGameTimeSinceCreation) (+ _offsetspeed (Variables|Default|GetRandom_0)))) (Math|Trig|Sin(Degrees) (* (Actor|GetGameTimeSinceCreation) (+ _offsetspeed (Variables|Default|GetRandom_1))))) (- (Math|Vector|MakeVector (Variables|Default|GetRandom_2) (Variables|Default|GetRandom_3) (Variables|Default|GetRandom_4)) "1.500000,1.500000,1.500000")) (Variables|Default|GetOffsetAmplitude)) false false)
  (Transformation|SetRelativeRotation _cloud (Math|Conversions|RotationFromXVector (* (+ (Math|Vector|MakeVector (Math|Trig|Sin(Degrees) (* (Actor|GetGameTimeSinceCreation) (+ _rotationspeed (Variables|Default|GetRandom_2)))) (Math|Trig|Sin(Degrees) (* (Actor|GetGameTimeSinceCreation) (+ _rotationspeed (Variables|Default|GetRandom_3)))) (Math|Trig|Sin(Degrees) (* (Actor|GetGameTimeSinceCreation) (+ _rotationspeed (Variables|Default|GetRandom_4))))) (Math|Vector|MakeVector (Variables|Default|GetRandom) (Variables|Default|GetRandom_0) (Variables|Default|GetRandom_1))) "360.000000,360.000000,360.000000")) false false))

(fn ConstructionScript)