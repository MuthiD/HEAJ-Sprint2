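; Gameplay game mode that sets up the shared camera for all player controllers and handles the end of a match.
; On BeginPlay it sets game-only input, points every controller at the gameplay camera and stores the controllers in the game instance.
; GameOver opens the game-over level, while a once-only Win saves non-hidden players' one-based controller IDs to the game instance before opening the win level.
; SaveWinners is an unfinished stub.
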(event Custom|GameOver
  (Game|OpenLevel(byObjectReference) "/Game/Levels/L_GameOver.L_GameOver"))

(event Custom|Win
  (Utilities|FlowControl|DoOnce false
    (:Completed
      (bind _outactors (Actor|GetAllActorsOfClass "/Game/Blueprints/Gameplay/Pawn/BP_GAMEPLAY_Pawn_Player.BP_GAMEPLAY_Pawn_Player_C"))
      (for _array_element _outactors
        (if (not (Variables|/Script/Engine.Actor|GetbHidden _array_element))
          (bind _asbp_gameplay_controller (Utilities|Casting|CastToBP_GAMEPLAY_Controller (Pawn|GetController _array_element)))
          (Utilities|Array|Add (Variables|Default|GetId_Winners) (+ (Class|GameplayStatics|GetPlayerControllerID _asbp_gameplay_controller) 1))))
      (Default|SetWinners (Variables|Default|GetAs%20BP%20Sprint%202%20Gameinstance) (Variables|Default|GetId_Winners))
      (Game|OpenLevel(byObjectReference) "/Game/Levels/L_Win.L_Win"))))

(event Custom|SaveWinners
  (Utilities|Casting|CastToBP_Sprint2_Gameinstance (Game|GetGameInstance)))

(event EventBeginPlay
  (Input|SetInputModeGameOnly (Game|GetPlayerController 0) false)
  (bind _returnvalue (Actor|GetActorOfClass "/Game/Blueprints/Gameplay/Pawn/BP_GAMEPLAY_Camera.BP_GAMEPLAY_Camera_C"))
  (Variables|Default|SetBP_Camera _returnvalue)
  (bind _outactors (Actor|GetAllActorsOfClass "/Game/Blueprints/Gameplay/Controller/BP_GAMEPLAY_Controller.BP_GAMEPLAY_Controller_C"))
  (bind _output_get (Variables|Default|SetArrayController _outactors))
  (for _array_element _output_get
    (Game|Player|SetViewTargetwithBlend _array_element (Variables|Default|GetBP_Camera) 0.0 "VTBlend_Linear" 0.0 false))
  (bind _asbp_sprint_2_gameinstance (Utilities|Casting|CastToBP_Sprint2_Gameinstance (Game|GetGameInstance)))
  (bind _output_get_2 (Variables|Default|SetAs%20BP%20Sprint%202%20Gameinstance _asbp_sprint_2_gameinstance))
  (Variables|/Game/Blueprints/BP_Sprint2_Gameinstance.BP_Sprint2_Gameinstance_C|SetPlayersController _output_get_2 (Variables|Default|GetArrayController)))

(fn ConstructionScript)