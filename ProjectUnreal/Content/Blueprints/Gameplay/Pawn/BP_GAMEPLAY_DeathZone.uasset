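; Death zone that eliminates players entering its box and triggers game over when all are eliminated.
; An overlapping player pawn is hidden and has its input disabled, with the hidden flag serving as the death state.
; Each elimination scans all player pawns, clearing AllHide if any is visible; the flag is never reset here.
; If AllHide remains true, it calls GameOver on the cached gamemode after a short delay.
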(event OnComponentBeginOverlap(Box)
  (params (OverlappedComponent :type Primitive%20Component%20Object%20Reference) (OtherActor :type Actor%20Object%20Reference) (OtherComp :type Primitive%20Component%20Object%20Reference) (OtherBodyIndex :type Integer) (bFromSweep :type Boolean) (SweepResult :type Hit%20Result%20Structure%20%28by%20ref%29))
  (bind _asbp_gameplay_pawn_player (Utilities|Casting|CastToBP_GAMEPLAY_Pawn_Player OtherActor))
  (Rendering|SetActorHiddenInGame _asbp_gameplay_pawn_player true)
  (Input|DisableInput _asbp_gameplay_pawn_player 0)
  (CallFunction|VerifNbPlayerALife))

(event Custom|VerifNbPlayerALife
  (bind _outactors (Actor|GetAllActorsOfClass "/Game/Blueprints/Gameplay/Pawn/BP_GAMEPLAY_Pawn_Player.BP_GAMEPLAY_Pawn_Player_C"))
  (bind _array_element (Utilities|Array|ForEachLoopwithBreak _outactors :!label _label)
    (:LoopBody
      (if (not (Variables|/Script/Engine.Actor|GetbHidden _array_element))
        (Variables|Default|SetAllHide? false)
        (goto _label Break)))
    (:Completed
      (if (Variables|Default|GetAllHide?)
        (Utilities|FlowControl|Delay 0.5)
        (Default|GameOver (Variables|Default|Get%20GAMEPLAY%20Gamemode))))))

(event EventBeginPlay
  (bind _asbp_gameplay_gamemode (Utilities|Casting|CastToBP_GAMEPLAY_Gamemode (Game|GetGameMode)))
  (Variables|Default|Set%20GAMEPLAY%20Gamemode _asbp_gameplay_gamemode))

(fn ConstructionScript)