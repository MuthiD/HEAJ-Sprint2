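; Master Blueprint for falling item hazards that knock the player back on contact and despawn after a set lifetime.
; On BeginPlay it waits DelayLife, then destroys itself.
; When its Box overlaps a player pawn, it launches that character opposite its facing direction, scaled by ForceRecul, overriding horizontal velocity only.
; Other overlapping actors only have their names printed.
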(event OnComponentBeginOverlap(Box)
  (params (OverlappedComponent :type Primitive%20Component%20Object%20Reference) (OtherActor :type Actor%20Object%20Reference) (OtherComp :type Primitive%20Component%20Object%20Reference) (OtherBodyIndex :type Integer) (bFromSweep :type Boolean) (SweepResult :type Hit%20Result%20Structure%20%28by%20ref%29))
  (bind _asbp_gameplay_pawn_player (Utilities|Casting|CastToBP_GAMEPLAY_Pawn_Player OtherActor)
    (:then
      (Character|LaunchCharacter _asbp_gameplay_pawn_player (* (Math|Vector|NegateVector (Transformation|GetActorForwardVector _asbp_gameplay_pawn_player)) (* (Variables|Default|GetForceRecul) 1e+02)) true false))
    (:CastFailed
      (Development|PrintString (Utilities|GetDisplayName OtherActor)))))

(event EventBeginPlay
  (Utilities|FlowControl|Delay (Variables|Default|GetDelayLife))
  (Actor|DestroyActor))

(fn ConstructionScript)