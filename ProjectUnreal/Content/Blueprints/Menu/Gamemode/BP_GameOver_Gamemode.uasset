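; Game mode for the game over screen that initializes player state and restores saved audio volume.
; On BeginPlay, only if the first player state's Name is empty, it calls that state's SetVariables, then LoadVolumeSound.
; LoadVolumeSound sets the base sound mix and applies BP_SaveGame's volume array as class overrides by index: both VFX and Music, then each separately, so later entries override the first.
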(event EventBeginPlay
  (bind _asbp_sprint_2_playerstate (Utilities|Casting|CastToBP_Sprint2_Playerstate (Utilities|Array|Get(acopy) (Variables|/Script/Engine.GameStateBase|GetPlayerArray (Game|GetGameState)))))
  (if (Utilities|Enum|Equal(Enum) (Variables|/Game/Blueprints/BP_Sprint2_Playerstate.BP_Sprint2_Playerstate_C|GetName _asbp_sprint_2_playerstate) "")
    (Default|SetVariables _asbp_sprint_2_playerstate)
    (CallFunction|LoadVolumeSound)))

(fn ConstructionScript)

(fn LoadVolumeSound
  (Class|GameplayStatics|SetBaseSoundMix "/Game/Sounds/SCM_MainSoundMix.SCM_MainSoundMix")
  (bind _returnvalue (SaveGame|DoesSaveGameExist "BP_SaveGame"))
  (if _returnvalue
    (bind _returnvalue_2 (SaveGame|LoadGamefromSlot "BP_SaveGame"))
    (bind _asbp_save_game (Utilities|Casting|CastToBP_SaveGame _returnvalue_2))
    (for (_array_element _array_index) (Variables|/Game/Blueprints/BP_SaveGame.BP_SaveGame_C|GetSoundVolume _asbp_save_game)
      (switch int _array_index
        (:0
          (Audio|SetSoundMixClassOverride "/Game/Sounds/SCM_MainSoundMix.SCM_MainSoundMix" "/Game/Sounds/Class/SC_VFX.SC_VFX" _array_element 1.0 0.0 true)
          (Audio|SetSoundMixClassOverride "/Game/Sounds/SCM_MainSoundMix.SCM_MainSoundMix" "/Game/Sounds/Class/SC_Music.SC_Music" _array_element 1.0 0.0 true))
        (:1
          (Audio|SetSoundMixClassOverride "/Game/Sounds/SCM_MainSoundMix.SCM_MainSoundMix" "/Game/Sounds/Class/SC_VFX.SC_VFX" _array_element 1.0 0.0 true))
        (:2
          (Audio|SetSoundMixClassOverride "/Game/Sounds/SCM_MainSoundMix.SCM_MainSoundMix" "/Game/Sounds/Class/SC_Music.SC_Music" _array_element 1.0 0.0 true))))))