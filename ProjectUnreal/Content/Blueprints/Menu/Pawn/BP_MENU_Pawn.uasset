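; Menu pawn that turns Enhanced Input presses into lobby screen actions.
; On BeginPlay it adds the IMC_Menu mapping context, then caches the menu GameMode and finds the menu HUD actor through the GameMode's HUD class.
; Input actions forward directly to the HUD's lobby widget to add or remove a player, launch the game or go back to the menu.
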(event Input|EnhancedActionEvents|EnhancedInputActionIA_Valid
  (params (ActionValue :type Boolean) (ElapsedSeconds :type Float%20%28double-precision%29) (TriggeredSeconds :type Float%20%28double-precision%29) (InputAction :type Input%20Action%20Object%20Reference :default "/Game/Blueprints/Menu/Controller/Input/Action/IA_Valid.IA_Valid"))
  (:Started
    (Default|LaunchGame (Variables|/Game/Blueprints/Menu/Hud/BP_MENU_Hud.BP_MENU_Hud_C|GetWBP_Lobby (Variables|Default|GetAs%20BP%20MENU%20Hud)))))

(event Input|EnhancedActionEvents|EnhancedInputActionIA_BackMenu
  (params (ActionValue :type Boolean) (ElapsedSeconds :type Float%20%28double-precision%29) (TriggeredSeconds :type Float%20%28double-precision%29) (InputAction :type Input%20Action%20Object%20Reference :default "/Game/Blueprints/Menu/Controller/Input/Action/IA_BackMenu.IA_BackMenu"))
  (:Started
    (Default|BackMenu (Variables|/Game/Blueprints/Menu/Hud/BP_MENU_Hud.BP_MENU_Hud_C|GetWBP_Lobby (Variables|Default|GetAs%20BP%20MENU%20Hud)))))

(event Input|EnhancedActionEvents|EnhancedInputActionIA_NbPlayerSuivant
  (params (ActionValue :type Boolean) (ElapsedSeconds :type Float%20%28double-precision%29) (TriggeredSeconds :type Float%20%28double-precision%29) (InputAction :type Input%20Action%20Object%20Reference :default "/Game/Blueprints/Menu/Controller/Input/Action/IA_NbPlayerSuivant.IA_NbPlayerSuivant"))
  (:Started
    (Default|AddPlayer (Variables|/Game/Blueprints/Menu/Hud/BP_MENU_Hud.BP_MENU_Hud_C|GetWBP_Lobby (Variables|Default|GetAs%20BP%20MENU%20Hud)))))

(event Input|EnhancedActionEvents|EnhancedInputActionIA_NbPlayerPrecedent
  (params (ActionValue :type Boolean) (ElapsedSeconds :type Float%20%28double-precision%29) (TriggeredSeconds :type Float%20%28double-precision%29) (InputAction :type Input%20Action%20Object%20Reference :default "/Game/Blueprints/Menu/Controller/Input/Action/IA_NbPlayerPrecedent.IA_NbPlayerPrecedent"))
  (:Started
    (Default|RemovePlayer (Variables|/Game/Blueprints/Menu/Hud/BP_MENU_Hud.BP_MENU_Hud_C|GetWBP_Lobby (Variables|Default|GetAs%20BP%20MENU%20Hud)))))

(event EventBeginPlay
  (bind _asplayer_controller (Utilities|Casting|CastToPlayerController (Pawn|GetController)))
  (Utilities|IsValid (PlayerController|LocalPlayerSubsystems|GetEnhancedInputLocalPlayerSubsystem _asplayer_controller)
    (:Is%20Valid
      (Input|AddMappingContext (PlayerController|LocalPlayerSubsystems|GetEnhancedInputLocalPlayerSubsystem _asplayer_controller) "/Game/Blueprints/Menu/Controller/Input/IMC_Menu.IMC_Menu" 0 "(bIgnoreAllPressedKeysUntilRelease=True,bForceImmediately=False,bNotifyUserSettings=False)")
      (bind _asbp_menu_gamemode (Utilities|Casting|CastToBP_MENU_Gamemode (Game|GetGameMode)))
      (bind _output_get (Variables|Default|SetAs%20BP%20MENU%20Gamemode _asbp_menu_gamemode))
      (bind _returnvalue (Actor|GetActorOfClass (Variables|/Script/Engine.GameModeBase|GetHUDClass _output_get)))
      (bind _asbp_menu_hud (Utilities|Casting|CastToBP_MENU_Hud _returnvalue))
      (Variables|Default|SetAs%20BP%20MENU%20Hud _asbp_menu_hud))))

(fn ConstructionScript)