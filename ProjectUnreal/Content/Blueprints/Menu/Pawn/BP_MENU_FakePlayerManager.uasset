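; BP_MENU_FakePlayerManager spawns stand-in BP_FakePlayer actors in the menu to represent players.
; One tick after BeginPlay, it spawns one for player controller 0 through SpawnFakePlayer.
; That event picks a spawn transform by controller ID, passes name, color and skeletal mesh from BP_Sprint2_Playerstate, and stores the new actor back on that player state.
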(event Custom|SpawnFakePlayer
  (params (PlayerState :type BP%20Sprint%202%20Playerstate%20Object%20Reference))
  (bind _returnvalue (Game|SpawnActorfromClass "/Game/Blueprints/Menu/Pawn/BP_FakePlayer.BP_FakePlayer_C" (Utilities|Array|Get(acopy) (Variables|Default|GetFake%20Player%20Spawn) (Class|GameplayStatics|GetPlayerControllerID (Game|GetPlayerController PlayerState))) "Undefined" "MultiplyWithRoot" 0 (Utilities|Struct|MakeSTRUCT_PlayerData (Variables|/Game/Blueprints/BP_Sprint2_Playerstate.BP_Sprint2_Playerstate_C|GetName PlayerState) (Variables|/Game/Blueprints/BP_Sprint2_Playerstate.BP_Sprint2_Playerstate_C|GetColor PlayerState) (Variables|/Game/Blueprints/BP_Sprint2_Playerstate.BP_Sprint2_Playerstate_C|GetSkeletal PlayerState)) 0))
  (Variables|/Game/Blueprints/BP_Sprint2_Playerstate.BP_Sprint2_Playerstate_C|SetFakePlayer PlayerState _returnvalue))

(event EventBeginPlay
  (Utilities|FlowControl|DelayUntilNextTick)
  (bind _asbp_sprint_2_playerstate (Utilities|Casting|CastToBP_Sprint2_Playerstate (Variables|/Script/Engine.Controller|GetPlayerState (Game|GetPlayerController 0))))
  (CallFunction|SpawnFakePlayer _asbp_sprint_2_playerstate))

(fn ConstructionScript)