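; BP_MENU_Controller is the controller for the menu, setting up split-screen and input when play begins.
; On BeginPlay it force-disables split-screen, then checks its player controller ID.
; Controllers with a non-zero ID have their input disabled.
; The ID 0 controller adds the IMC_Menu mapping context to its Enhanced Input subsystem, so only that player drives the menu.
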(event EventBeginPlay
  (bind _self self)
  (bind _returnvalue (PlayerController|LocalPlayerSubsystems|GetEnhancedInputLocalPlayerSubsystem _self))
  (Class|GameplayStatics|SetForceDisableSplitscreen true)
  (if (not (== (Class|GameplayStatics|GetPlayerControllerID self) 0))
    (Input|DisableInput self)
    (else
      (Utilities|IsValid _returnvalue
        (:Is%20Valid
          (Input|AddMappingContext _returnvalue "/Game/Blueprints/Menu/Controller/Input/IMC_Menu.IMC_Menu" 0 "(bIgnoreAllPressedKeysUntilRelease=True,bForceImmediately=False,bNotifyUserSettings=False)"))))))

(fn ConstructionScript)