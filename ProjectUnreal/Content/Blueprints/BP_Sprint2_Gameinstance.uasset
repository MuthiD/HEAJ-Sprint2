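; BP_Sprint2_Gameinstance is a game instance that manages local multiplayer players and stores a player list.
; AddPlayer spawns a local player and controller, adds the IMC_Menu input mapping, initializes its BP_Sprint2_Playerstate, and reports success with that state.
; RemovePlayer removes the last local controller and its pawn while more than one remains.
; SetPlayerList and GetPlayerList write and read the stored Players list.
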(event EventSetPlayerList
  (params (Players :type Array%20of%20STRUCT%20Player%20Data%20Structures))
  (Variables|Default|SetPlayers Players))

(event EventRemovePlayer
  (if (> (Class|GameplayStatics|GetNumLocalPlayerControllers) 1)
    (Class|GameplayStatics|RemovePlayer (Game|GetPlayerController (- (Class|GameplayStatics|GetNumLocalPlayerControllers) 1)) true)))

(fn AddPlayer
  (bind _returnvalue (Class|GameplayStatics|CreatePlayer -1))
  (Input|AddMappingContext (PlayerController|LocalPlayerSubsystems|GetEnhancedInputLocalPlayerSubsystem _returnvalue) "/Game/Blueprints/Menu/Controller/Input/IMC_Menu.IMC_Menu" 0 "(bIgnoreAllPressedKeysUntilRelease=True,bForceImmediately=False,bNotifyUserSettings=False)")
  (bind _asbp_sprint_2_playerstate (Utilities|Casting|CastToBP_Sprint2_Playerstate (Variables|/Script/Engine.Controller|GetPlayerState _returnvalue)))
  (Default|SetVariables _asbp_sprint_2_playerstate)
  (return (> (Class|GameplayStatics|GetNumLocalPlayerControllers) 1) _asbp_sprint_2_playerstate))

(fn GetPlayerList
  (return (Variables|Default|GetPlayers)))