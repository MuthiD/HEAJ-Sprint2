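; Player state Blueprint that holds each local player's name and visual identity: skeletal mesh, anim blueprint, icon and player materials.
; SetVariables derives the name and one of four DT_Player rows (Joueur1-4) from the current player controller count, then caches that row's assets.
; GetPlayerInfos returns the cached values to callers.
; When destroyed, it also destroys its FakePlayer actor if valid.
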(event Custom|SetVariables
  (Variables|Default|SetName (Utilities|String|Append "Player " (Utilities|String|ToString(Integer) (Class|GameplayStatics|GetNumPlayerControllers))))
  (bind _returnvalue (Utilities|GetDataTableRow "/Game/Blueprints/DataTable/DT_Player.DT_Player" (Utilities|Select :Index (- (Class|GameplayStatics|GetNumPlayerControllers) 1) :Option%200 "Joueur1" :Option%201 "Joueur2" :Option%202 "Joueur3" :Option%203 "Joueur4"))
    (:then
      (Variables|Default|SetSkeletal (.skeletal _returnvalue))
      (Variables|Default|SetABP (.abp _returnvalue))
      (Variables|Default|SetMat_Icone (.mat_icone _returnvalue))
      (Variables|Default|SetMat_Player (.mat_players _returnvalue)))))

(event EventDestroyed
  (bind _fakeplayer (Variables|Default|GetFakePlayer)
    (:then
      (Actor|DestroyActor _fakeplayer))
    (:else)))

(fn ConstructionScript)

(fn GetPlayerInfos
  (return (Variables|Default|GetName) (Variables|Default|GetSkeletal) (Variables|Default|GetABP) (Variables|Default|GetMat_Icone) (Variables|Default|GetMat_Player)))