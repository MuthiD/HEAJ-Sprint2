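; Blueprint function library that saves each player's identity and appearance to the GameInstance and restores it, likely to carry it across level changes.
; SavePlayerState packs name, skeletal mesh, anim blueprint and icon material from every BP_Sprint2_Playerstate into a struct array, sent through interface messages.
; SetDataPlayerInStruct reads that array back and applies entries by PlayerArray index, so restoration depends on matching player order.
; The SaveScore input is unused.
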(fn SavePlayerState
  (params (SaveScore? :type Boolean))
  (for _array_element (Variables|/Script/Engine.GameStateBase|GetPlayerArray (Game|GetGameState))
    (bind _asbp_sprint_2_playerstate (Utilities|Casting|CastToBP_Sprint2_Playerstate _array_element))
    (Utilities|Array|Add (LocalVariables|GetPlayerData) (Utilities|Struct|MakeSTRUCT_PlayerData (Variables|/Game/Blueprints/BP_Sprint2_Playerstate.BP_Sprint2_Playerstate_C|GetName _asbp_sprint_2_playerstate) (Variables|/Game/Blueprints/BP_Sprint2_Playerstate.BP_Sprint2_Playerstate_C|GetSkeletal _asbp_sprint_2_playerstate) (Variables|/Game/Blueprints/BP_Sprint2_Playerstate.BP_Sprint2_Playerstate_C|GetABP _asbp_sprint_2_playerstate) (Variables|/Game/Blueprints/BP_Sprint2_Playerstate.BP_Sprint2_Playerstate_C|GetMat_Icone _asbp_sprint_2_playerstate))))
  (Class|BPIGameinstance|SetPlayerList(Message) (Game|GetGameInstance) (LocalVariables|GetPlayerData)))

(fn SetDataPlayerinStruct
  (bind _players (Class|BPIGameinstance|GetPlayerList(Message) (Game|GetGameInstance)))
  (bind _output_get (LocalVariables|SetPlayerData _players))
  (if (> (Utilities|Array|Length _output_get) 0)
    (for (_array_element _array_index) (Variables|/Script/Engine.GameStateBase|GetPlayerArray (Game|GetGameState))
      (bind _asbp_sprint_2_playerstate (Utilities|Casting|CastToBP_Sprint2_Playerstate _array_element))
      (Variables|/Game/Blueprints/BP_Sprint2_Playerstate.BP_Sprint2_Playerstate_C|SetName _asbp_sprint_2_playerstate (.name (Utilities|Array|Get(acopy) (LocalVariables|GetPlayerData) _array_index)))
      (Variables|/Game/Blueprints/BP_Sprint2_Playerstate.BP_Sprint2_Playerstate_C|SetSkeletal _asbp_sprint_2_playerstate (.skeletalmeshaa (Utilities|Array|Get(acopy) (LocalVariables|GetPlayerData) _array_index)))
      (Variables|/Game/Blueprints/BP_Sprint2_Playerstate.BP_Sprint2_Playerstate_C|SetABP _asbp_sprint_2_playerstate (.abp (Utilities|Array|Get(acopy) (LocalVariables|GetPlayerData) _array_index)))
      (Variables|/Game/Blueprints/BP_Sprint2_Playerstate.BP_Sprint2_Playerstate_C|SetMat_Icone _asbp_sprint_2_playerstate (.mat_icone (Utilities|Array|Get(acopy) (LocalVariables|GetPlayerData) _array_index))))))